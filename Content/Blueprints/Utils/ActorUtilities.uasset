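; Utility function library for filtering objects and toggling actors on or off.
; IsSpecific tests an object against a comparison mode: any, a given actor, an actor tag, or a class.
; SetEnabled switches an actor's visibility, collision and tick together, then mutes or unmutes its audio components.
; Audio is toggled by setting each component's VolumeMultiplier to zero or full, so original volume values are not preserved.
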(fn IsSpecific
  (params (Object :type Actor%20Object%20Reference) (Comparison :type E_DetectionSelection%20Enum :default "NewEnumerator0") (Actor :type Actor%20Object%20Reference) (Tag :type Name) (Class :type Actor%20Class%20Reference))
  (switch Utilities|FlowControl|Switch|SwitchonE_DetectionSelection Comparison
    (:NewEnumerator0
      (return true))
    (:NewEnumerator3
      (return (== Object Actor)))
    (:NewEnumerator1
      (bind _asactor (Utilities|Casting|CastToActor Object)
        (:then
          (return (Actor|ActorHasTag _asactor Tag)))
        (:CastFailed
          (return false))))
    (:NewEnumerator2
      (return (Class|GameplayStatics|ObjectIsA Object Class)))))

(fn SetEnabled
  (params (enabled :type Boolean) (Actor :type Actor%20Object%20Reference))
  (Rendering|SetActorHiddenInGame Actor (not enabled))
  (Collision|SetActorEnableCollision Actor enabled)
  (Actor|Tick|SetActorTickEnabled Actor enabled)
  (Actor|SetActorAudioComponentsEnabled Actor enabled))

(fn SetActorAudioComponentsEnabled
  (params (Target :type Actor%20Object%20Reference) (Enabled :type Boolean))
  (for _array_element (Actor|GetComponentsByClass Target "/Script/Engine.AudioComponent")
    (if Enabled
      (Variables|/Script/Engine.AudioComponent|SetVolumeMultiplier _array_element 1.0)
      (else
        (Variables|/Script/Engine.AudioComponent|SetVolumeMultiplier _array_element 0.0)))))