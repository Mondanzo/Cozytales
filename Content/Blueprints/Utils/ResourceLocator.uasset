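; ResourceLocator is a utility Blueprint that looks up shared game resources for other code.
; Get Quest Manager casts the current game state to BP_GameState and returns its QuestManagerRef.
; Get Player Key linearly scans the DT_CM_KeyLookup data table and returns the key from the first row whose input action matches the one passed in.
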(fn GetQuestManager
  (bind _asbp_game_state (Utilities|Casting|CastToBP_GameState (Game|GetGameState (LocalVariables|Get__WorldContext))))
  (return (Variables|/Game/Blueprints/Systems/BP_GameState.BP_GameState_C|GetQuestManagerRef _asbp_game_state)))

(fn GetPlayerKey
  (params (InputAction :type Input%20Action%20Object%20Reference))
  (bind _outrownames (DataTable|GetDataTableRowNames "/Game/Assets/UI/Prompts/DT_CM_KeyLookup.DT_CM_KeyLookup"))
  (for _array_element _outrownames
    (bind _returnvalue (Utilities|GetDataTableRow "/Game/Assets/UI/Prompts/DT_CM_KeyLookup.DT_CM_KeyLookup" _array_element)
      (:then
        (if (== (.inputaction _returnvalue) InputAction)
          (return (.key _returnvalue)))))))