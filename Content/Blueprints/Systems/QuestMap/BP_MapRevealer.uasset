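; BP_MapRevealer is a component that uncovers the quest map around its owner by painting into a render target.
; Once the owner moves past a distance threshold, it stamps a reveal texture at the position mapped through BP_LevelCapture2D.
; Events clear the target to black to reset or white to reveal everything, with a reset on BeginPlay.
; Revealed state saves per slot as an EXR in SaveGames and is redrawn on load.
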(event Custom|Paint
  (bind _returnvalue (Components|GetOwner))
  (bind _returnvalue_2 (Transformation|GetActorLocation _returnvalue))
  (bind _returnvalue_3 (Math|Conversions|ToVector2D(Vector) _returnvalue_2))
  (Variables|Default|SetLast%20Capture%20Position _returnvalue_3)
  (bind (_canvas _size _context) (Rendering|BeginDrawCanvastoRenderTarget (Variables|Default|GetTexture)))
  (Canvas|DrawTexture :self _canvas :RenderTexture "/Game/Blueprints/Systems/QuestMap/T_RevealTexture.T_RevealTexture" :ScreenPosition (- (* _size (Default|WorldtoPercentages (Variables|Default|GetMap%20Center) _returnvalue_3)) (/ (Variables|Default|GetReveal%20Size) 2.0)) :ScreenSize (Math|Conversions|ToVector2D(Vector) (Variables|Default|GetReveal%20Size)) :CoordinateSize "(X=1.000000,Y=1.000000)" :PivotPoint "(X=0.500000,Y=0.500000)")
  (Rendering|EndDrawCanvastoRenderTarget _context))

(event Custom|Reset%20Map
  (Rendering|ClearRenderTarget2D (Variables|Default|GetTexture)))

(event Custom|Reveal%20Full%20Map
  (Rendering|ClearRenderTarget2D (Variables|Default|GetTexture) "(R=1.000000,G=1.000000,B=1.000000,A=1.000000)"))

(event EventBeginPlay
  (bind _returnvalue (Actor|GetActorOfClass "/Game/Blueprints/Systems/QuestMap/BP_LevelCapture2D.BP_LevelCapture2D_C"))
  (Variables|Default|SetMap%20Center _returnvalue)
  (Rendering|ClearRenderTarget2D (Variables|Default|GetTexture))
  (CallFunction|Paint))

(event EventTick
  (params (DeltaSeconds :type Float%20%28single-precision%29))
  (if (> (Math|Vector|Distance2D(Vector) (Variables|Default|GetLast%20Capture%20Position) (Math|Conversions|ToVector2D(Vector) (Transformation|GetActorLocation (Components|GetOwner)))) (Variables|Default|GetDistance))
    (CallFunction|Paint)))

(event Custom|CustomEvent
  (params (bSuccess :type Boolean))
  (Development|PrintString (Utilities|String|Append "Saved? " (Utilities|String|ToString(Boolean) bSuccess))))

(event Custom|Save%20Texture
  (params (Slot%20Name :type String))
  (bind _returnvalue (Class|KismetSystemLibrary|GetProjectSavedDirectory))
  (bind _returnvalue_2 (Utilities|String|Append Slot%20Name ".exr"))
  (bind _array (Utilities|Array|MakeArray _returnvalue "SaveGames" _returnvalue_2))
  (bind _returnvalue_3 (Class|BlueprintPathsLibrary|Combine _array))
  ;[1 1 1] Save Texture
  (Class|ImageWriteBlueprintLibrary|ExporttoDisk (Variables|Default|GetTexture) _returnvalue_3 (Utilities|Struct|MakeImageWriteOptions "EXR" (delegate Custom|CustomEvent)))
  (Development|PrintString (Utilities|String|Append "saved to " _returnvalue_3)))

(event Custom|Load%20Texture
  (params (Slot%20Name :type String))
  (bind _returnvalue (Class|KismetSystemLibrary|GetProjectSavedDirectory))
  (bind _returnvalue_2 (Utilities|String|Append Slot%20Name ".exr"))
  (bind _texture (Variables|Default|GetTexture))
  (bind (_width _height) (Class|CanvasRenderTarget2D|GetSize _texture))
  (bind _array (Utilities|Array|MakeArray _returnvalue "SaveGames" _returnvalue_2))
  (bind _returnvalue_3 (Class|BlueprintPathsLibrary|Combine _array))
  ;[1 1 1] Load Texture
  (if (Class|BlueprintPathsLibrary|FileExists _returnvalue_3)
    (bind _returnvalue_4 (Class|KismetRenderingLibrary|ImportFileasTexture2D _returnvalue_3))
    (bind (_canvas _size _context) (Rendering|BeginDrawCanvastoRenderTarget (Variables|Default|GetTexture)))
    (Canvas|DrawTexture :self _canvas :RenderTexture _returnvalue_4 :ScreenPosition "(X=0.000000,Y=0.000000)" :ScreenSize (Math|Vector2D|MakeVector2D (Math|Conversions|ToFloat(Integer) _width) (Math|Conversions|ToFloat(Integer) _height)) :CoordinateSize "(X=1.000000,Y=1.000000)" :BlendMode "BLEND_Opaque" :PivotPoint "(X=0.500000,Y=0.500000)")
    (Rendering|EndDrawCanvastoRenderTarget _context)))