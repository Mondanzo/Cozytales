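; Orthographic scene-capture actor for the quest map that renders the level to a texture and converts between world and map coordinates.
; Render hides actors matching TagsToHide, captures once, then clears the hidden list.
; Conversions pass through normalized percentages, assuming a square area from OrthoWidth and texture SizeX, with rotation fixed at zero.
; MapToWorld calls PercentagesToMap instead of MapToPercentages, so it multiplies by map size rather than dividing.
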(event Custom|Render
  (for _array_element (Variables|Default|GetTags%20To%20Hide)
    (bind _outactors (Actor|GetAllActorswithTag _array_element))
    (for _array_element_2 _outactors
      (Class|SceneCaptureComponent|HideActorComponents (Variables|DecalActor|GetCaptureComponent2D) _array_element_2 true)))
  (Rendering|SceneCapture|CaptureScene (Variables|DecalActor|GetCaptureComponent2D) :!class /Script/Engine.SceneCaptureComponent2D)
  (Class|SceneCaptureComponent|ClearHiddenComponents (Variables|DecalActor|GetCaptureComponent2D)))

(fn ConstructionScript)

(fn WorldtoMap
  (params (World%20Position :type Vector%202D%20Structure))
  (return (CallFunction|PercentagestoMap (CallFunction|WorldtoPercentages World%20Position))))

(fn MaptoWorld
  (params (Map%20Position :type Vector%202D%20Structure))
  (return (CallFunction|PercentagestoWorld (CallFunction|PercentagestoMap Map%20Position))))

(fn WorldtoPercentages
  (params (World%20Position :type Vector%202D%20Structure))
  (return (/ (+ (Class|KismetMathLibrary|GetRotated2D (- World%20Position (Math|Conversions|ToVector2D(Vector) (Transformation|GetActorLocation))) 0.0) (CallFunction|GetWorldHalfSize)) (CallFunction|GetWorldFullSize))))

(fn MaptoPercentages
  (params (Map%20Position :type Vector%202D%20Structure))
  (return (/ Map%20Position (CallFunction|GetMapFullSize))))

(fn PercentagestoWorld
  (params (Percentages :type Vector%202D%20Structure))
  (return (+ (Class|KismetMathLibrary|GetRotated2D (- (* Percentages (CallFunction|GetWorldFullSize)) (CallFunction|GetWorldHalfSize)) 0.0) (Math|Conversions|ToVector2D(Vector) (Transformation|GetActorLocation)))))

(fn PercentagestoMap
  (params (Percentages :type Vector%202D%20Structure))
  (return (* Percentages (CallFunction|GetMapFullSize))))

(fn GetWorldHalfSize
  (return (/ (CallFunction|GetWorldFullSize) 2.0)))

(fn GetWorldFullSize
  (bind _capturecomponent2d (Variables|DecalActor|GetCaptureComponent2D))
  (bind _orthowidth (Variables|/Script/Engine.SceneCaptureComponent2D|GetOrthoWidth _capturecomponent2d))
  (return (Math|Vector2D|MakeVector2D _orthowidth _orthowidth)))

(fn GetMapHalfSize
  (return (/ (CallFunction|GetMapFullSize) 2.0)))

(fn GetMapFullSize
  (bind _capturecomponent2d (Variables|DecalActor|GetCaptureComponent2D))
  (bind _texturetarget (Variables|/Script/Engine.SceneCaptureComponent2D|GetTextureTarget _capturecomponent2d))
  (bind _sizex (Variables|/Script/Engine.TextureRenderTarget2D|GetSizeX _texturetarget))
  (bind _returnvalue (Math|Conversions|ToFloat(Integer) _sizex))
  (return (Math|Vector2D|MakeVector2D _returnvalue _returnvalue)))