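; Game state Blueprint that runs the day cycle clock and triggers periodic autosaves.
; Tick advances CurrentDaytime by DaySpeed and broadcasts it through the DaytimeUpdated dispatcher, which the state also binds to itself to reset the value to zero at 360.
; A looping timer started on BeginPlay calls AutoSave every few seconds, which passes the save request to BP_GameInstance.
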(event Custom|Event%20AutoSave
  ;[0.2402 0.2814 1] Start Autosave Timer
  (CallFunction|AutoSave))

(event Custom|Event%20OnDaytimeUpdated
  (params (NewDaytime :type Float%20%28double-precision%29))
  (if (>= NewDaytime 3.6e+02)
    (Variables|Default|SetCurrentDaytime 0.0)))

(event EventBeginPlay
  (EventDispatchers|BindEventtoDaytimeUpdated (delegate Custom|Event%20OnDaytimeUpdated))
  ;[0.2402 0.2814 1] Start Autosave Timer
  (Utilities|Time|SetTimerbyEvent (delegate Custom|Event%20AutoSave) 5.0 true))

(event EventTick
  (params (DeltaSeconds :type Float%20%28single-precision%29))
  (bind _output_get (Variables|Default|SetCurrentDaytime (+ (* DeltaSeconds (Variables|Default|GetDaySpeed)) (Variables|Default|GetCurrentDaytime))))
  (Default|CallDaytimeUpdated _output_get))

(fn ConstructionScript)

(fn AutoSave
  (bind _asbp_game_instance (Utilities|Casting|CastToBP_GameInstance (Game|GetGameInstance)))
  (Default|EventSaveGame _asbp_game_instance))