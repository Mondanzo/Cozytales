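; BP_MySaveGame is a save game object that persists the player's transform and quest status.
; Its SaveGame event copies both values into its own variables, then writes itself to the slot given by its SaveSlotName and UserIndex.
; LoadGame reads that slot, casts the result to BP_MySaveGame and returns the stored values from the loaded instance without copying them onto itself.
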(event Custom|Event%20SaveGame
  (params (CurrentPlayerTrf :type Transform) (CurrentQuestStatus :type Array%20of%20S%20Quest%20Structures))
  (Variables|DataToSave|SetPlayerTransform CurrentPlayerTrf)
  (Variables|DatatoSave|SetQuestStatus CurrentQuestStatus)
  (SaveGame|SaveGametoSlot self (Variables|SaveGameIDVars|GetSaveSlotName) (Variables|SaveGameIDVars|GetUserIndex)))

(fn LoadGame
  (bind _returnvalue (SaveGame|LoadGamefromSlot (Variables|SaveGameIDVars|GetSaveSlotName) (Variables|SaveGameIDVars|GetUserIndex)))
  (bind _asbp_my_save_game (Utilities|Casting|CastToBP_MySaveGame _returnvalue))
  (return (Variables|BP_MySaveGame_C|GetPlayerTransform _asbp_my_save_game) (Variables|BP_MySaveGame_C|GetQuestStatus _asbp_my_save_game)))