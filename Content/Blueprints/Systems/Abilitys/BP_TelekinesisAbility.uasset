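; Telekinesis ability that lets the player grab, move and rotate physics-simulated objects in view.
; A camera line trace hands the hit component to a physics handle, pulls the spring arm in, and starts a looping timer holding it along the view direction.
; Mouse wheel changes hold distance, look input rotates in rotation mode, and releasing input resets everything.
; A separate ControlWind trace only prints on "Wind Controller" actors.
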(event Custom|Control%20Wind
  (bind _playercamera (Variables|Default|GetPlayerCamera))
  (bind _returnvalue (Transformation|GetWorldLocation _playercamera))
  ;[1 1 1] Wind Controller
  (bind (_outhit _returnvalue_2) (Collision|LineTraceByChannel _returnvalue (+ _returnvalue (* (Math|Vector|GetForwardVector (Transformation|GetWorldRotation _playercamera)) 1e+03)) "TraceTypeQuery1" false 0 "None"))
  (if _returnvalue_2
    (if (Actor|ActorHasTag (.HitActor (Collision|BreakHitResult _outhit)) "Wind Controller")
      (Development|PrintText "I am A Wind Controller"))))

(event Custom|Grab
  (bind _playercamera (Variables|Default|GetPlayerCamera))
  (bind _returnvalue (Transformation|GetWorldLocation _playercamera))
  ;[0.05098 0.05098 0.05098] Telekinesis
  (bind (_outhit _returnvalue_2) (Collision|LineTraceByChannel _returnvalue (+ _returnvalue (* (Math|Vector|GetForwardVector (Transformation|GetWorldRotation _playercamera)) 1e+03)) "TraceTypeQuery1" false 0 "None"))
  (if _returnvalue_2
    (Variables|Default|SetGrabDistance (.Distance (Collision|BreakHitResult _outhit)))
    (Variables|Default|SetGrabRotation (Transformation|GetWorldRotation (.HitComponent (Collision|BreakHitResult _outhit))))
    (if (Physics|IsSimulatingPhysics (.HitComponent (Collision|BreakHitResult _outhit)) "None")
      (Variables|/Script/Engine.SpringArmComponent|SetTargetArmLength (Variables|Default|GetPlayerSpringArm) -1e+01)
      (Physics|Components|PhysicsHandle|GrabComponentatLocationwithRotation (Variables|Default|GetPlayerPhysicHandler) (.HitComponent (Collision|BreakHitResult _outhit)) "None" (Transformation|GetWorldLocation (.HitComponent (Collision|BreakHitResult _outhit))) (Transformation|GetWorldRotation (.HitComponent (Collision|BreakHitResult _outhit))))
      (Variables|Default|SetGrabbing? true)
      (bind _returnvalue_3 (Utilities|Time|SetTimerbyEvent (delegate Custom|SetGrabLocation) 0.01 true))
      (Variables|Default|SetGrabTimeHandle _returnvalue_3))))

(event Custom|SetGrabLocation
  (bind _playercamera (Variables|Default|GetPlayerCamera))
  ;[0.05098 0.05098 0.05098] Telekinesis
  (Class|PhysicsHandleComponent|SetTargetLocationandRotation (Variables|Default|GetPlayerPhysicHandler) (+ (Transformation|GetWorldLocation _playercamera) (* (Math|Vector|GetForwardVector (Transformation|GetWorldRotation _playercamera)) (Variables|Default|GetGrabDistance))) (Variables|Default|GetGrabRotation)))

(event Input|EnhancedActionEvents|EnhancedInputActionIA_Telekinesis_RotationMode
  (params (ActionValue :type Boolean) (ElapsedSeconds :type Float%20%28double-precision%29) (TriggeredSeconds :type Float%20%28double-precision%29) (InputAction :type Input%20Action%20Object%20Reference :default "/Game/Input/Actions/IA_Telekinesis_RotationMode.IA_Telekinesis_RotationMode"))
  (bind _grabbing_ (Variables|Default|GetGrabbing?))
  ;[1 1 1] Telekinesis-Input
  (:Triggered
    (if _grabbing_
      (Variables|Default|SetRotateMode true)))
  (:Completed
    (if _grabbing_
      (Variables|Default|SetRotateMode false))))

(event Input|EnhancedActionEvents|EnhancedInputActionIA_Telekinesis
  (params (ActionValue :type Boolean) (ElapsedSeconds :type Float%20%28double-precision%29) (TriggeredSeconds :type Float%20%28double-precision%29) (InputAction :type Input%20Action%20Object%20Reference :default "/Game/Input/Actions/IA_Telekinesis.IA_Telekinesis"))
  ;[1 1 1] Telekinesis-Input
  (:Triggered
    (CallFunction|Grab))
  (:Completed
    (CallFunction|DeactivateAbility)))

(event Input|EnhancedActionEvents|EnhancedInputActionIA_Look
  (params (ActionValue :type Vector%202D%20Structure) (ElapsedSeconds :type Float%20%28double-precision%29) (TriggeredSeconds :type Float%20%28double-precision%29) (InputAction :type Input%20Action%20Object%20Reference :default "/Game/Input/Actions/IA_Look.IA_Look"))
  ;[1 1 1] Telekinesis-Input
  (if (Variables|Default|GetRotateMode)
    (Variables|Default|SetGrabRotation (Math|Rotator|MakeRotator 0.0 (+ (.y ActionValue) (.pitch (Variables|Default|GetGrabRotation))) (+ (.yaw (Variables|Default|GetGrabRotation)) (.x ActionValue))))))

(event Input|MouseEvents|MouseWheelDown
  (params (Key :type Key%20Structure))
  ;[1 1 1] Telekinesis-Input
  (:Pressed
    (Variables|Default|SetGrabDistance (Math|Float|Clamp(Float) (+ (Variables|Default|GetGrabDistance) -5e+01) 5.5e+02 1e+03))))

(event Input|MouseEvents|MouseWheelUp
  (params (Key :type Key%20Structure))
  ;[1 1 1] Telekinesis-Input
  (:Pressed
    (Variables|Default|SetGrabDistance (Math|Float|Clamp(Float) (+ (Variables|Default|GetGrabDistance) 5e+01) 2e+02 1e+03))))

(fn DeactivateAbility
  (Physics|Components|PhysicsHandle|ReleaseComponent (Variables|Default|GetPlayerPhysicHandler))
  (Utilities|Time|ClearandInvalidateTimerbyHandle (Variables|Default|GetGrabTimeHandle))
  (Variables|Default|SetGrabbing? false)
  (Variables|/Script/Engine.SpringArmComponent|SetTargetArmLength (Variables|Default|GetPlayerSpringArm) 3e+02)
  (Variables|Default|SetRotateMode false))