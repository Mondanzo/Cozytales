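; BP_SpecialQuestMarker is a quest area marker that reports whether a 2D location lies within MaxDistance while it is active.
; It registers with the quest manager one tick after BeginPlay, exposes its QuestID list, and toggles IsActive on quest activation events.
; ShouldBeEnabled destroys the actor if any linked quest has a particular status; its other status check is unreachable.
; The construction script scales a tall cylinder to match the radius.
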(event EventQuestActivated
  (Variables|Default|SetIsActive true))

(event EventQuestDeactivated
  (Variables|Default|SetIsActive false))

(event EventBeginPlay
  (Utilities|FlowControl|DelayUntilNextTick)
  (Default|RegisterQuestElement (CallFunction|GetQuestManager) self))

(fn ConstructionScript
  (bind _max_distance (Variables|Default|GetMax%20Distance))
  (bind _returnvalue (/ _max_distance 2e+02))
  (Transformation|SetRelativeScale3D (Variables|Default|GetCylinder) (Math|Vector|MakeVector _returnvalue _returnvalue 1e+02)))

(fn WithinRange
  (params (Location :type Vector%202D%20Structure))
  (return (and (<= (Math|Vector|Distance2D(Vector) Location (Math|Conversions|ToVector2D(Vector) (Transformation|GetActorLocation))) (Variables|Default|GetMax%20Distance)) (Variables|Default|GetIsActive))))

(fn ShouldbeEnabled
  (for _array_element (Variables|Default|GetQuestID)
    (bind _quest (Default|GetQuestfromArray(ID) (CallFunction|GetQuestManager) _array_element))
    (if (Utilities|Enum|Equal(Enum) (.QuestStatus (Utilities|Struct|BreakS_Quest _quest)) "NewEnumerator4")
      (Actor|DestroyActor)
      (return false))))

(fn GetAssociatedQuests
  (return (Variables|Default|GetQuestID)))