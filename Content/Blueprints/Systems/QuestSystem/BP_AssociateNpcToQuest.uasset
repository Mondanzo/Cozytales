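; Quest-linked component that changes an owning BP_BaseNPC's conversations when its quest activates or deactivates, as chosen by OnActivate.
; On BeginPlay, after a short delay, it checks the first QuestID's state to catch up, updating for an already succeeded or active quest and notifying the NPC if active.
; A one-shot update pushes configured dialogues, monologues, removals and talk partner into the NPC's conversation manager.
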(event EventQuestActivated
  (if (Variables|Default|GetOnActivate?)
    (CallFunction|UpdateQuestDialogues)))

(event EventQuestDeactivated
  (|CallParentFunction)
  (Development|PrintString (Utilities|String|ToString(Text) (Utilities|Text|FormatText "{DisplayName}: Associate NPC Event Quest Deactivated for ID {ID}" (Utilities|GetDisplayName (Components|GetOwner)) (Utilities|Array|Get(acopy) (Variables|Default|GetQuestID)))) true true "(R=1.000000,G=0.007126,B=0.000000,A=1.000000)" 5.0)
  (if (not (Variables|Default|GetOnActivate?))
    (CallFunction|UpdateQuestDialogues)))

(event EventBeginPlay
  (Utilities|FlowControl|Delay 0.5)
  (|CallParentFunction)
  (bind _status (CallFunction|GetQuestState (Utilities|Array|Get(acopy) (Variables|Default|GetQuestID))))
  (switch Utilities|FlowControl|Switch|SwitchonE_QuestStatus _status
    (:NewEnumerator1
      (if (Variables|Default|GetOnActivate?)
        (CallFunction|UpdateQuestDialogues))
      (bind _asbp_base_npc (Utilities|Casting|CastToBP_BaseNPC (Components|GetOwner)))
      (Default|EventonAssociatedEventAlreadyActive _asbp_base_npc))
    (:NewEnumerator4
      (CallFunction|UpdateQuestDialogues))))

(fn UpdateQuestDialogues
  (if (not (Variables|Default|GetHas%20Triggered))
    (Variables|Default|SetHas%20Triggered true)
    (bind _asbp_base_npc (Utilities|Casting|CastToBP_BaseNPC (Components|GetOwner)))
    (Default|AddNewPassiveDialogues (Variables|/Game/Blueprints/Characters/NPCCharacter/BP_BaseNPC.BP_BaseNPC_C|GetBPC_ConversationManager _asbp_base_npc) (Variables|Default|GetPassiveDialoguesToAdd))
    (Default|AddNewPassiveMonologues (Variables|/Game/Blueprints/Characters/NPCCharacter/BP_BaseNPC.BP_BaseNPC_C|GetBPC_ConversationManager _asbp_base_npc) (Variables|Default|GetPassiveMonologuesToAdd))
    (Default|SetActiveDialogue (Variables|/Game/Blueprints/Characters/NPCCharacter/BP_BaseNPC.BP_BaseNPC_C|GetBPC_ConversationManager _asbp_base_npc) (Variables|Default|GetActiveDialogueToSet))
    (Default|RemoveConversations (Variables|/Game/Blueprints/Characters/NPCCharacter/BP_BaseNPC.BP_BaseNPC_C|GetBPC_ConversationManager _asbp_base_npc) (Variables|Default|GetConversationsToRemove))
    (Default|SetActiveTalkPartner (Variables|/Game/Blueprints/Characters/NPCCharacter/BP_BaseNPC.BP_BaseNPC_C|GetBPC_ConversationManager _asbp_base_npc) (Variables|Default|GetActiveTalkPartnerToSet))))