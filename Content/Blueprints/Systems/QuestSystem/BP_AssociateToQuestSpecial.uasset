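; Component that ties a special forge quest NPC (BP_NPCForg_QuestSpecial) to quest states, enabling or disabling it as those quests change.
; ShouldBeEnabled checks each quest ID's status against spawn, hide and persist flags, combined by AND or any-match.
; When enabled, it overrides the NPC's valid, invalid and missing dialogues, per-outcome quest complete/activate/deactivate settings and marker tag.
; It unregisters from the quest manager on EndPlay.
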(event EventEndPlay
  (params (EndPlayReason :type EEndPlayReason%20Enum :default "Destroyed"))
  (bind _asi_quest_associated (Utilities|Casting|CastToI_QuestAssociated self))
  (Default|UnregisterQuestElement (CallFunction|GetQuestManager) _asi_quest_associated))

(event EventQuestActivated
  (bind _new_tag (Variables|Default|GetNew%20Tag))
  (bind _available (CallFunction|ShouldbeEnabled))
  (CallFunction|SetEnabled _available (Components|GetOwner))
  (if _available
    (bind _special_npc (Variables|Default|GetSpecial%20NPC)
      (:then
        (Utilities|FlowControl|Sequence
          (:then_0
            (bind _new_invalid_dialogue (Variables|Default|GetNew%20Invalid%20Dialogue)
              (:then
                (Variables|/Game/Blueprints/Characters/NPCCharacter/BP_NPCForg_QuestSpecial.BP_NPCForg_QuestSpecial_C|SetQuestMapInvalidSpecialDialogue _special_npc _new_invalid_dialogue))
              (:else)))
          (:then_1
            (bind _new_valid_dialogue (Variables|Default|GetNew%20Valid%20Dialogue)
              (:then
                (Variables|/Game/Blueprints/Characters/NPCCharacter/BP_NPCForg_QuestSpecial.BP_NPCForg_QuestSpecial_C|SetQuestMapValidSpecialDialogue _special_npc _new_valid_dialogue))
              (:else)))
          (:then_2
            (bind _new_missing_dialogue (Variables|Default|GetNew%20Missing%20Dialogue)
              (:then
                (Variables|/Game/Blueprints/Characters/NPCCharacter/BP_NPCForg_QuestSpecial.BP_NPCForg_QuestSpecial_C|SetQuestMapMissingSpecialDialogue _special_npc _new_missing_dialogue))
              (:else)))
          (:then_3
            (Utilities|FlowControl|Sequence
              (:then_0
                (Variables|/Game/Blueprints/Characters/NPCCharacter/BP_NPCForg_QuestSpecial.BP_NPCForg_QuestSpecial_C|SetCompleteQuestInvalid _special_npc (Variables|Default|GetComplete%20Quest%20Invalid)))
              (:then_1
                (Variables|/Game/Blueprints/Characters/NPCCharacter/BP_NPCForg_QuestSpecial.BP_NPCForg_QuestSpecial_C|SetCompleteQuestValid _special_npc (Variables|Default|GetComplete%20Quest%20Valid)))
              (:then_2
                (Variables|/Game/Blueprints/Characters/NPCCharacter/BP_NPCForg_QuestSpecial.BP_NPCForg_QuestSpecial_C|SetCompleteQuestMissing _special_npc (Variables|Default|GetComplete%20Quest%20Missing)))
              (:then_3
                (Variables|/Game/Blueprints/Characters/NPCCharacter/BP_NPCForg_QuestSpecial.BP_NPCForg_QuestSpecial_C|SetDeactivateQuestInvalid _special_npc (Variables|Default|GetDisable%20Quest%20Invalid)))
              (:then_4
                (Variables|/Game/Blueprints/Characters/NPCCharacter/BP_NPCForg_QuestSpecial.BP_NPCForg_QuestSpecial_C|SetDeactivateQuestValid _special_npc (Variables|Default|GetDisable%20Quest%20Valid)))
              (:then_5
                (Variables|/Game/Blueprints/Characters/NPCCharacter/BP_NPCForg_QuestSpecial.BP_NPCForg_QuestSpecial_C|SetDeactivateQuestMissing _special_npc (Variables|Default|GetDisable%20Quest%20Missing)))
              (:then_6
                (Variables|/Game/Blueprints/Characters/NPCCharacter/BP_NPCForg_QuestSpecial.BP_NPCForg_QuestSpecial_C|SetActivateQuestInvalid _special_npc (Variables|Default|GetActivate%20Quest%20Invalid)))
              (:then_7
                (Variables|/Game/Blueprints/Characters/NPCCharacter/BP_NPCForg_QuestSpecial.BP_NPCForg_QuestSpecial_C|SetActivateQuestValid _special_npc (Variables|Default|GetActivate%20Quest%20Valid)))
              (:then_8
                (Variables|/Game/Blueprints/Characters/NPCCharacter/BP_NPCForg_QuestSpecial.BP_NPCForg_QuestSpecial_C|SetActivateQuestMissing _special_npc (Variables|Default|GetActivate%20Quest%20Missing)))
              (:then_9
                (if (!= _new_tag "")
                  (Variables|/Game/Blueprints/Characters/NPCCharacter/BP_NPCForg_QuestSpecial.BP_NPCForg_QuestSpecial_C|SetSpecialMarkerTag _special_npc _new_tag)))))))
      (:else))))

(event EventBeginPlay
  (bind _asbp_npcforg_quest_special (Utilities|Casting|CastToBP_NPCForg_QuestSpecial (Components|GetOwner)))
  (Variables|Default|SetSpecial%20NPC _asbp_npcforg_quest_special)
  (Utilities|FlowControl|DelayUntilNextTick)
  (CallFunction|QuestActivated))

(event EventQuestDeactivated
  (bind _new_tag (Variables|Default|GetNew%20Tag))
  (bind _available (CallFunction|ShouldbeEnabled))
  (CallFunction|SetEnabled _available (Components|GetOwner))
  (if _available
    (bind _special_npc (Variables|Default|GetSpecial%20NPC)
      (:then
        (Utilities|FlowControl|Sequence
          (:then_0
            (bind _new_invalid_dialogue (Variables|Default|GetNew%20Invalid%20Dialogue)
              (:then
                (Variables|/Game/Blueprints/Characters/NPCCharacter/BP_NPCForg_QuestSpecial.BP_NPCForg_QuestSpecial_C|SetQuestMapInvalidSpecialDialogue _special_npc _new_invalid_dialogue))
              (:else)))
          (:then_1
            (bind _new_valid_dialogue (Variables|Default|GetNew%20Valid%20Dialogue)
              (:then
                (Variables|/Game/Blueprints/Characters/NPCCharacter/BP_NPCForg_QuestSpecial.BP_NPCForg_QuestSpecial_C|SetQuestMapValidSpecialDialogue _special_npc _new_valid_dialogue))
              (:else)))
          (:then_2
            (bind _new_missing_dialogue (Variables|Default|GetNew%20Missing%20Dialogue)
              (:then
                (Variables|/Game/Blueprints/Characters/NPCCharacter/BP_NPCForg_QuestSpecial.BP_NPCForg_QuestSpecial_C|SetQuestMapMissingSpecialDialogue _special_npc _new_missing_dialogue))
              (:else)))
          (:then_3
            (Utilities|FlowControl|Sequence
              (:then_0
                (Variables|/Game/Blueprints/Characters/NPCCharacter/BP_NPCForg_QuestSpecial.BP_NPCForg_QuestSpecial_C|SetCompleteQuestInvalid _special_npc (Variables|Default|GetComplete%20Quest%20Invalid)))
              (:then_1
                (Variables|/Game/Blueprints/Characters/NPCCharacter/BP_NPCForg_QuestSpecial.BP_NPCForg_QuestSpecial_C|SetCompleteQuestValid _special_npc (Variables|Default|GetComplete%20Quest%20Valid)))
              (:then_2
                (Variables|/Game/Blueprints/Characters/NPCCharacter/BP_NPCForg_QuestSpecial.BP_NPCForg_QuestSpecial_C|SetCompleteQuestMissing _special_npc (Variables|Default|GetComplete%20Quest%20Missing)))
              (:then_3
                (Variables|/Game/Blueprints/Characters/NPCCharacter/BP_NPCForg_QuestSpecial.BP_NPCForg_QuestSpecial_C|SetDeactivateQuestInvalid _special_npc (Variables|Default|GetDisable%20Quest%20Invalid)))
              (:then_4
                (Variables|/Game/Blueprints/Characters/NPCCharacter/BP_NPCForg_QuestSpecial.BP_NPCForg_QuestSpecial_C|SetDeactivateQuestValid _special_npc (Variables|Default|GetDisable%20Quest%20Valid)))
              (:then_5
                (Variables|/Game/Blueprints/Characters/NPCCharacter/BP_NPCForg_QuestSpecial.BP_NPCForg_QuestSpecial_C|SetDeactivateQuestMissing _special_npc (Variables|Default|GetDisable%20Quest%20Missing)))
              (:then_6
                (Variables|/Game/Blueprints/Characters/NPCCharacter/BP_NPCForg_QuestSpecial.BP_NPCForg_QuestSpecial_C|SetActivateQuestInvalid _special_npc (Variables|Default|GetActivate%20Quest%20Invalid)))
              (:then_7
                (Variables|/Game/Blueprints/Characters/NPCCharacter/BP_NPCForg_QuestSpecial.BP_NPCForg_QuestSpecial_C|SetActivateQuestValid _special_npc (Variables|Default|GetActivate%20Quest%20Valid)))
              (:then_8
                (Variables|/Game/Blueprints/Characters/NPCCharacter/BP_NPCForg_QuestSpecial.BP_NPCForg_QuestSpecial_C|SetActivateQuestMissing _special_npc (Variables|Default|GetActivate%20Quest%20Missing)))
              (:then_9
                (if (!= _new_tag "")
                  (Variables|/Game/Blueprints/Characters/NPCCharacter/BP_NPCForg_QuestSpecial.BP_NPCForg_QuestSpecial_C|SetSpecialMarkerTag _special_npc _new_tag)))))))
      (:else))))

(fn ShouldbeEnabled
  (bind _quest_manager (CallFunction|GetQuestManager))
  (bind _and (Variables|Default|GetAND))
  (bind _array_element (Utilities|Array|ForEachLoopwithBreak (Variables|Default|GetQuestID) :!label _label)
    (:LoopBody
      (Utilities|IsValid _quest_manager
        (:Is%20Valid
          (bind _quest (Default|GetQuestfromArray(ID) _quest_manager _array_element))
          (if (Math|Boolean|ORBoolean (Math|Boolean|ANDBoolean (Utilities|Enum|Equal(Enum) (.QuestStatus (Utilities|Struct|BreakS_Quest _quest)) "NewEnumerator1") (not (Variables|Default|GetSpawnOnlyOnceQuestIsCompleted?)) (not (Variables|Default|GetHideForQuest))) (Math|Boolean|ANDBoolean (Utilities|Enum|Equal(Enum) (.QuestStatus (Utilities|Struct|BreakS_Quest _quest)) "NewEnumerator0") (Variables|Default|GetSpawnFromStart) (not (Utilities|Enum|Equal(Enum) (.QuestStatus (Utilities|Struct|BreakS_Quest _quest)) "NewEnumerator4"))) (and (Utilities|Enum|Equal(Enum) (.QuestStatus (Utilities|Struct|BreakS_Quest _quest)) "NewEnumerator4") (and (or (Variables|Default|GetSpawnOnlyOnceQuestIsCompleted?) (Variables|Default|GetShouldPersistAfterQuestIsDone?)) (not (Variables|Default|GetHideForQuest)))))
            (LocalVariables|SetQuest%20Available true)
            (if (not _and)
              (goto _label Break))
            (else
              (LocalVariables|SetQuest%20Not%20Available true)
              (if _and
                (goto _label Break)))))))
    (:Completed
      (return (and (LocalVariables|GetQuest%20Available) (not (LocalVariables|GetQuest%20Not%20Available)))))))

(fn CheckifAllAssociatedQuestsAreDone
  (for _array_element (Variables|Default|GetQuestID)
    (bind _quest (Default|GetQuestfromArray(ID) (CallFunction|GetQuestManager) _array_element))
    (if (Utilities|Enum|NotEqual(Enum) (.QuestStatus (Utilities|Struct|BreakS_Quest _quest)) "NewEnumerator4")
      (return false)))
  (return true))

(fn GetAssociatedQuests
  (return (Variables|Default|GetQuestID)))