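; Quest marker actor that defines a circular area around its location for the quest identified by QuestID.
; After a short BeginPlay delay, it sets its active state from that quest's status or destroys itself, then registers with the quest manager through I_QuestAssociated.
; Activation events enable it, while deactivation destroys it.
; WithinRange does a 2D distance test against MaxDistance while active, and the construction script scales a tall cylinder to that radius.
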(event EventQuestDeactivated
  (Actor|DestroyActor))

(event EventQuestActivated
  (Variables|Default|SetIsActive true))

(event EventBeginPlay
  (Utilities|FlowControl|Delay 0.2)
  (bind _available (CallFunction|ShouldbeEnabled))
  (if _available
    (CallFunction|QuestActivated)
    (else
      (Variables|Default|SetIsActive false)))
  (bind _asi_quest_associated (Utilities|Casting|CastToI_QuestAssociated self))
  (Default|RegisterQuestElement (CallFunction|GetQuestManager) _asi_quest_associated))

(fn ConstructionScript
  (bind _max_distance (Variables|Default|GetMax%20Distance))
  (bind _returnvalue (/ _max_distance 2e+02))
  (Transformation|SetRelativeScale3D (Variables|Default|GetCylinder) (Math|Vector|MakeVector _returnvalue _returnvalue 1e+02)))

(fn WithinRange
  (params (Location :type Vector%202D%20Structure))
  (return (and (<= (Math|Vector|Distance2D(Vector) Location (Math|Conversions|ToVector2D(Vector) (Transformation|GetActorLocation))) (Variables|Default|GetMax%20Distance)) (Variables|Default|GetIsActive))))

(fn ShouldbeEnabled
  (bind _quest (Default|GetQuestfromArray(ID) (CallFunction|GetQuestManager) (Variables|Default|GetQuestID)))
  (if (Utilities|Enum|Equal(Enum) (.QuestStatus (Utilities|Struct|BreakS_Quest _quest)) "NewEnumerator4")
    (Actor|DestroyActor)
    (return false)
    (else
      (return (Utilities|Enum|Equal(Enum) (.QuestStatus (Utilities|Struct|BreakS_Quest _quest)) "NewEnumerator1")))))

(fn GetAssociatedQuests
  (return (Utilities|Array|MakeArray (Variables|Default|GetQuestID))))