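; Quest manager that tracks quest states, judges map markers handed in at the quest board, and plays result UI and sound.
; Loads quests from a DataTable, then reapplies statuses after notifying the GameInstance.
; Status updates activate or deactivate registered quest elements.
; After a delay, marker IDs resolve as success, failure or empty; failures start a reset timer, and NPC conversation managers get completion events by quest ID.
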(event Custom|CheckMarkerPlacement
  (params (QuestID :type Integer))
  (CallFunction|CheckQuestLocation QuestID))

(event Custom|OnQuestFailed
  (Development|PrintString "QUEST FAIL: WRONG LOCATION!  
SET NPC FAIL DIALOGUE" true true "(R=1.000000,G=0.000000,B=0.021536,A=1.000000)" 2e+01)
  (Default|PlayFailed (Variables|Default|Getquest_ui_ref))
  (Audio|SpawnSoundatLocation "/Game/Sounds/MetaSounds/MSP_QuestFailed.MSP_QuestFailed" (Transformation|GetActorLocation (Game|GetPlayerCharacter 0)) "0, 0, 0" 1.0 1.0 0.0 0 0))

(event Custom|OnQuestSuccesed
  (Development|PrintString "QUEST COMPLEATE: LOCATION CORRECT! 
SET NPC SUCCES DIALOGUE" true true "(R=0.000000,G=1.000000,B=0.097885,A=1.000000)" 2e+01)
  (Default|PlaySuccessful (Variables|Default|Getquest_ui_ref))
  (Audio|SpawnSoundatLocation "/Game/Sounds/MetaSounds/MSP_QuestSuccess.MSP_QuestSuccess" (Transformation|GetActorLocation (Game|GetPlayerCharacter 0)) "0, 0, 0" 1.0 1.0 0.0 0 0))

(event Custom|OnQuestEmpty
  (Development|PrintString "QUEST FAIL: NO QUEST MARKER!  
SET A QUEST MARKER PLZ" true true "(R=1.000000,G=0.000000,B=0.021536,A=1.000000)" 2e+01)
  (Default|PlayFailed (Variables|Default|Getquest_ui_ref))
  (Audio|SpawnSoundatLocation "/Game/Sounds/MetaSounds/MSP_QuestFailed.MSP_QuestFailed" (Transformation|GetActorLocation (Game|GetPlayerCharacter 0)) "0, 0, 0" 1.0 1.0 0.0 0 0))

(event Custom|Event%20SetQuestOnBoard
  (params (Map :type WBP%20Player%20Map%20Object%20Reference))
  (Development|PrintString "SetQuestOnBoard Timer Started" true true "(R=0.000000,G=0.660000,B=1.000000,A=1.000000)" 1e+01 "")
  (bind _questid (Default|GetQuestMarkerResult Map))
  (Default|EventonMapHandedin Map)
  (Utilities|FlowControl|Delay (Variables|Default|GetQuestAcceptedTime))
  (CallFunction|CheckMarkerPlacement _questid))

(event Custom|Event%20ActivateQuest
  (params (QuestID :type Integer))
  (Development|PrintString (Utilities|String|Append (Utilities|String|MakeLiteralString "Quest was activated! ID: ") (Utilities|String|ToString(Integer) QuestID)))
  (CallFunction|UpdateQuestStatus QuestID "NewEnumerator1"))

(event Custom|Event%20StartFailStateResetTimer
  (params (Fail%20ID :type Integer))
  (Development|PrintString "Fail State Timer Started!")
  (Utilities|FlowControl|Delay 3e+02)
  (Development|PrintString "Fail State Expired")
  (CallFunction|UpdateQuestStatus Fail%20ID "NewEnumerator0"))

(event EventBeginPlay
  (CallFunction|InitializeQuests)
  (CallFunction|SetupWidget)
  (Utilities|FlowControl|DelayUntilNextTick)
  ;[1 0.4129 0.2708] Check if Game was loaded
  (bind _asbp_game_instance (Utilities|Casting|CastToBP_GameInstance (Game|GetGameInstance)))
  (Default|EventonQuestManagerFinishedLoading _asbp_game_instance)
  (Utilities|FlowControl|DelayUntilNextTick)
  (for _array_element (Variables|Default|GetQuestArray)
    (CallFunction|UpdateQuestStatus (.Quest_ID (Utilities|Struct|BreakS_Quest _array_element)) (.QuestStatus (Utilities|Struct|BreakS_Quest _array_element)))))

(fn ConstructionScript)

(fn InitializeQuests
  (bind _questdatatable (Variables|Default|GetQuestDataTable))
  (bind _outrownames (DataTable|GetDataTableRowNames _questdatatable))
  (for _array_element _outrownames
    (bind _returnvalue (Utilities|GetDataTableRow _questdatatable _array_element)
      (:then
        (Utilities|Array|Add (Variables|Default|GetQuestArray) _returnvalue)))))

(fn SetQuestMarkerPosition
  (params (Position :type Vector))
  (Variables|Default|SetQuestMarkerPosition Position))

(fn CheckQuestLocation
  (params (QuestID :type Integer))
  (bind _output_get (LocalVariables|SetIDQuest QuestID))
  (Development|PrintString (Utilities|String|ToString(Integer) _output_get) true true "(R=1.000000,G=0.000000,B=0.093626,A=1.000000)" 5.0)
  (if (<= _output_get 0)
    (switch int (LocalVariables|GetIDQuest)
      (:-2
        (CallFunction|OnQuestEmpty))
      (:-1
        (CallFunction|OnQuestFailed)))
    (CallFunction|HandleQuestFailState (LocalVariables|GetIDQuest))
    (else
      (CallFunction|UpdateQuestStatus (LocalVariables|GetIDQuest) "NewEnumerator4")
      (Development|PrintString "Quest status set  to OnBoard_Success")
      (CallFunction|OnQuestSuccesed)))
  (CallFunction|NotifyNpcsAboutQuestSuccess (LocalVariables|GetIDQuest)))

(fn UpdateQuestStatus
  (params (QuestID :type Integer) (NewStatus :type E_QuestStatus%20Enum :default "NewEnumerator0"))
  (bind (_quest _index) (CallFunction|GetQuestfromArray(ID) QuestID))
  (bind _structout (Utilities|Struct|SetmembersinS_Quest _quest NewStatus))
  (CallFunction|UpdateQuestfromArray _index _structout)
  (for _array_element (Variables|Default|GetRegistered%20Elements)
    (Utilities|IsValid (Utilities|ToObject(Interface) _array_element)
      (:Is%20Valid
        (bind _quest_id (Default|GetAssociatedQuests _array_element))
        (if (and (Utilities|Array|ContainsItem _quest_id QuestID) (Utilities|Enum|Equal(Enum) NewStatus "NewEnumerator1"))
          (Default|QuestActivated _array_element)
          (else
            ;[0.04232 0.1218 0.2083] Checks whether the other quest is active or if it hasn't been activated yet, so that event actors don't get disabled, even though their assigned quest is active or was never started in the first place. -Andrei
            (for _array_element_2 _quest_id
              (bind _quest_2 (CallFunction|GetQuestfromArray(ID) _array_element_2))
              (if (and (Utilities|Enum|NotEqual(Enum) (Utilities|Struct|BreakS_Quest _quest_2) "NewEnumerator1") (Utilities|Enum|NotEqual(Enum) (Utilities|Struct|BreakS_Quest _quest_2) "NewEnumerator0"))
                (Default|QuestDeactivated _array_element)))))))))

(fn GetQuestfromArray(ID)
  (params (QuestID :type Integer))
  (for (_array_element _array_index) (Variables|Default|GetQuestArray)
    (if (== QuestID (.Quest_ID (Utilities|Struct|BreakS_Quest _array_element)))
      (return _array_element _array_index))))

(fn UpdateQuestfromArray
  (params (Index :type Integer) (New%20Item :type S%20Quest%20Structure))
  (Utilities|Array|SetArrayElem (Variables|Default|GetQuestArray) Index New%20Item))

(fn NotifyNpcsAboutQuestSuccess
  (params (QuestID :type Integer))
  (for _array_element (Variables|Default|GetQuestArray)
    (if (== (.Quest_ID (Utilities|Struct|BreakS_Quest _array_element)) QuestID)
      (for _array_element_2 (.WorldNpcConversationModification (Utilities|Struct|BreakS_Quest _array_element))
        (if (Utilities|Array|IsNotEmpty (Utilities|Struct|BreakS_QuestSuccessConvos _array_element_2))
          (CallFunction|UpdateWorldNpcsOfClass (Utilities|Struct|BreakS_QuestSuccessConvos _array_element_2) QuestID)
          (else
            (CallFunction|UpdateAllWorldNpcs QuestID)))))))

(fn UpdateAllWorldNpcs
  (params (QuestID :type Integer))
  (bind _outactors (Actor|GetAllActorsOfClass "/Game/Blueprints/Characters/NPCCharacter/BP_BaseNPC.BP_BaseNPC_C"))
  (for _array_element _outactors
    (Default|EventonQuestCompleted (Variables|/Game/Blueprints/Characters/NPCCharacter/BP_BaseNPC.BP_BaseNPC_C|GetBPC_ConversationManager _array_element) QuestID)))

(fn UpdateWorldNpcsOfClass
  (params (SelectedNpcs :type Array%20of%20BP%20Base%20NPC%20Class%20References) (QuestID :type Integer))
  (for _array_element SelectedNpcs
    (bind _outactors (Actor|GetAllActorsOfClass _array_element))
    (for _array_element_2 _outactors
      (Default|EventonQuestCompleted (Variables|/Game/Blueprints/Characters/NPCCharacter/BP_BaseNPC.BP_BaseNPC_C|GetBPC_ConversationManager _array_element_2) QuestID))))

(fn RegisterQuestElement
  (params (Target :type I%20Quest%20Associated%20Interface))
  (Utilities|Array|Add (Variables|Default|GetRegistered%20Elements) Target))

(fn UnregisterQuestElement
  (params (Quest%20Element :type I%20Quest%20Associated%20Interface))
  (bind _returnvalue (Utilities|Array|RemoveItem (Variables|Default|GetRegistered%20Elements) Quest%20Element))
  (if (not _returnvalue)
    (Development|PrintString "Failed to remove quest element!")))

(fn SetupWidget
  (bind _returnvalue (UserInterface|CreateWidget "/Game/UI/Widgets/WBP_QuestResult.WBP_QuestResult_C"))
  (UserInterface|Viewport|AddtoViewport _returnvalue 1)
  (Variables|Default|Setquest_ui_ref _returnvalue))

(fn HandleQuestFailState
  (params (FailID :type Integer))
  (CallFunction|UpdateQuestStatus FailID "NewEnumerator4")
  (CallFunction|EventStartFailStateResetTimer FailID))