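; Actor component for AI daily routines that picks the scheduled location matching the current time of day.
; It reads CurrentDaytime from BP_GameState and walks the Schedule map in key order, keeping the last location whose time has passed and stopping at the first later one.
; Map entries must therefore be in ascending time order; without a valid match, the first location is returned.
; A helper reports whether the schedule is empty.
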(fn GetCurrentScheduleLocation
  (bind _asbp_game_state (Utilities|Casting|CastToBP_GameState (Game|GetGameState)))
  (LocalVariables|SetGameState _asbp_game_state)
  (bind _values (Utilities|Map|Values (Variables|Default|GetSchedule)))
  (LocalVariables|SetScheduleLocations _values)
  (bind _keys (Utilities|Map|Keys (Variables|Default|GetSchedule)))
  (bind (_array_element _array_index) (Utilities|Array|ForEachLoopwithBreak _keys :!label _label)
    (:LoopBody
      (if (<= _array_element (Variables|/Game/Blueprints/Systems/BP_GameState.BP_GameState_C|GetCurrentDaytime (LocalVariables|GetGameState)))
        (LocalVariables|SetRetVal (Utilities|Array|Get(acopy) (LocalVariables|GetScheduleLocations) _array_index))
        (else
          (goto _label Break))))
    (:Completed
      (Utilities|IsValid (LocalVariables|GetRetVal)
        (:Is%20Valid
          (return (LocalVariables|GetRetVal)))
        (:Is%20Not%20Valid
          (return (Utilities|Array|Get(acopy) (LocalVariables|GetScheduleLocations))))))))

(fn IsScheduleEmpty?
  (return (Utilities|Map|IsEmpty (Variables|Default|GetSchedule))))