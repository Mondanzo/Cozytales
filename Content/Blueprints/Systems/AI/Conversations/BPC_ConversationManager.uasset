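; NPC component that holds a BP_BaseNPC's active dialogue and pools of passive dialogues and monologues.
; Line getters construct the active or a randomly picked conversation class to read its lines.
; On quest completion it scans DT_QuestsTable for changes affecting this NPC class, adds or removes conversations, then refreshes interaction priority.
; Additions under quest IDs -1 and -2 count as fail conversations, removed after a delay.
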(event Custom|Event%20OnFailConversationsAdded
  (params (AllFailConversations :type Array%20of%20BP%20Conversation%20P%20Class%20References))
  (Utilities|FlowControl|Delay (Variables|Default|GetPersistTimeForFailConversations))
  (CallFunction|RemoveConversations AllFailConversations))

(event Custom|Event%20OnQuestCompleted
  (params (QuestID :type Integer))
  (bind (_newdialogues _newmonologues _conversationstodelete) (CallFunction|GetConversationsRelatedtoQuest QuestID))
  (Utilities|FlowControl|Sequence
    (:then_0
      ;[0.1531 0.9303 1] Add new dialogues
      (CallFunction|AddNewPassiveDialogues _newdialogues))
    (:then_1
      ;[1 0.8549 0.3882] Add new monologues
      (CallFunction|AddNewPassiveMonologues _newmonologues))
    (:then_2
      ;[0.02745 0.05098 0.1137] Remove obsolete, event-related conversations
      (CallFunction|RemoveConversations _conversationstodelete))
    (:then_3
      ;[0.1771 0.1771 0.1771] Re-initialize InteractionPriority in case it was 0 before (or set it to 0 if all conversations have been removed)
      (bind _asbp_base_npc (Utilities|Casting|CastToBP_BaseNPC (Components|GetOwner)))
      (Default|InitializeInteractionPriority _asbp_base_npc))))

(event EventBeginPlay
  (bind _asbp_base_npc (Utilities|Casting|CastToBP_BaseNPC (Components|GetOwner)))
  (Variables|Default|SetOwner _asbp_base_npc))

(fn GetPassiveConversationLines
  (bind _possiblepassivedialogues (Variables|Passive|GetPossiblePassiveDialogues))
  (bind _returnvalue (Utilities|Array|Length _possiblepassivedialogues))
  (if (> _returnvalue 0)
    (bind _returnvalue_2 (Game|ConstructObjectfromClass (Utilities|Array|Get(acopy) (Variables|Passive|GetPossiblePassiveDialogues) (Math|Random|RandomIntegerinRange 0 (- _returnvalue 1)))))
    (return (Default|GetLines _returnvalue_2))))

(fn GetMonologueLines
  (bind _possiblemonologues (Variables|Passive|GetPossibleMonologues))
  (bind _returnvalue (Utilities|Array|Length _possiblemonologues))
  (if (> _returnvalue 0)
    (bind _returnvalue_2 (Game|ConstructObjectfromClass (Utilities|Array|Get(acopy) (Variables|Passive|GetPossibleMonologues) (Math|Random|RandomIntegerinRange 0 (- _returnvalue 1)))))
    (return (Default|GetLines _returnvalue_2))))

(fn GetConversationsRelatedtoQuest
  (params (QuestID :type Integer))
  (bind _outrownames (DataTable|GetDataTableRowNames "/Game/Blueprints/Systems/QuestSystem/DT_QuestsTable.DT_QuestsTable"))
  (bind _array_element (Utilities|Array|ForEachLoopwithBreak _outrownames)
    (:LoopBody
      (bind _returnvalue (Utilities|GetDataTableRow "/Game/Blueprints/Systems/QuestSystem/DT_QuestsTable.DT_QuestsTable" _array_element)
        (:then
          (if (== (.Quest_ID (Utilities|Struct|BreakS_Quest _returnvalue)) QuestID)
            (for _array_element_2 (.WorldNpcConversationModification (Utilities|Struct|BreakS_Quest _returnvalue))
              (if (Utilities|Array|IsEmpty (.AffectedNPCs (Utilities|Struct|BreakS_QuestSuccessConvos _array_element_2)))
                (for _array_element_3 (.PassiveDialoguesToAdd (Utilities|Struct|BreakS_QuestSuccessConvos _array_element_2)) :!label _label
                  (Utilities|Array|AddUnique (LocalVariables|GetRetDialogues) _array_element_3))
                (for _array_element_4 (.PassiveMonologuesToAdd (Utilities|Struct|BreakS_QuestSuccessConvos _array_element_2))
                  (Utilities|Array|AddUnique (LocalVariables|GetRetMonologues) _array_element_4))
                (for _array_element_5 (.ConversationsToDelete (Utilities|Struct|BreakS_QuestSuccessConvos _array_element_2))
                  (Utilities|Array|AddUnique (LocalVariables|GetRetToDelete) _array_element_5))
                (else
                  (bind _array_element_6 (Utilities|Array|ForEachLoopwithBreak (.AffectedNPCs (Utilities|Struct|BreakS_QuestSuccessConvos _array_element_2)))
                    (:LoopBody
                      (if (== _array_element_6 (Utilities|GetClass (Components|GetOwner)))
                        (goto _label)))))))
            (if (or (== QuestID -2) (== QuestID -1))
              (Utilities|FlowControl|Sequence
                (:then_0
                  (for _array_element_7 (LocalVariables|GetRetDialogues)
                    (Utilities|Array|AddUnique (LocalVariables|GetAllFailConversations) _array_element_7))
                  (for _array_element_8 (LocalVariables|GetRetMonologues)
                    (Utilities|Array|AddUnique (LocalVariables|GetAllFailConversations) _array_element_8))
                  (CallFunction|EventonFailConversationsAdded (LocalVariables|GetAllFailConversations)))))
            (return (LocalVariables|GetRetDialogues) (LocalVariables|GetRetMonologues) (LocalVariables|GetRetToDelete))))))))

(fn GetActiveConversationLines
  (if (Utilities|IsValidClass (Variables|Active(usingthesedisablespassiveconversationsforthisNPC!)|GetActiveDialogue))
    (bind _returnvalue (Game|ConstructObjectfromClass (Variables|Active(usingthesedisablespassiveconversationsforthisNPC!)|GetActiveDialogue)))
    (return (Default|GetLines _returnvalue) (Variables|/Game/Blueprints/Systems/AI/Conversations/BP_Conversation_P.BP_Conversation_P_C|GetQuestID _returnvalue))
    (else
      (return 0 -2))))

(fn AddNewPassiveDialogues
  (params (NewDialogues :type Array%20of%20BP%20Conversation%20P%20Class%20References))
  (for _array_element NewDialogues
    (Utilities|Array|AddUnique (Variables|Passive|GetPossiblePassiveDialogues) _array_element)))

(fn AddNewPassiveMonologues
  (params (Array :type Array%20of%20BP%20Conversation%20P%20Class%20References))
  (for _array_element Array
    (Utilities|Array|AddUnique (Variables|Passive|GetPossibleMonologues) _array_element)))

(fn RemoveConversations
  (params (Array :type Array%20of%20BP%20Conversation%20P%20Class%20References))
  (Utilities|FlowControl|Sequence
    (:then_0
      ;[0.3125 0.7832 1] Remove Passive Dialogues
      (for _array_element Array
        (if (Utilities|Array|ContainsItem (Variables|Passive|GetPossiblePassiveDialogues) _array_element)
          (Utilities|Array|RemoveItem (Variables|Passive|GetPossiblePassiveDialogues) _array_element))))
    (:then_1
      ;[1 0.8549 0.3882] Remove Passive Monologues
      (for _array_element_2 Array
        (if (Utilities|Array|ContainsItem (Variables|Passive|GetPossibleMonologues) _array_element_2)
          (Utilities|Array|RemoveItem (Variables|Passive|GetPossibleMonologues) _array_element_2))))
    (:then_2
      ;[0.02745 0.05098 0.1137] Remove Active Dialogue
      (for _array_element_3 Array
        (if (== _array_element_3 (Variables|Active(usingthesedisablespassiveconversationsforthisNPC!)|GetActiveDialogue))
          (Variables|Active(usingthesedisablespassiveconversationsforthisNPC!)|SetActiveDialogue 0))))))

(fn SetActiveDialogue
  (params (Active :type BP%20Conversation%20P%20Class%20Reference))
  (if (Utilities|IsValidClass Active)
    (Variables|Active(usingthesedisablespassiveconversationsforthisNPC!)|SetActiveDialogue Active)
    (Default|EventonNewActiveConversationSet (Variables|Default|GetOwner))))

(fn SetActiveTalkPartner
  (params (New%20Active%20Talk%20Partner :type BP%20Base%20NPC%20Object%20Reference))
  (Utilities|IsValid (Variables|Active(UsingTheseDisablesPassiveConversationsForThisNPC!)|GetActiveTalkPartner)
    (:Is%20Valid
      (Default|InvalidateActiveTalkPartner (Variables|Default|GetOwner)))
    (:Is%20Not%20Valid
      _))
  (Utilities|IsValid New%20Active%20Talk%20Partner
    (:Is%20Valid
      (Variables|Active(UsingTheseDisablesPassiveConversationsForThisNPC!)|SetActiveTalkPartner New%20Active%20Talk%20Partner)
      (Default|InitializeActiveDialogue (Variables|Default|GetOwner)))))

(fn HasValidActiveConversation?
  (return (Utilities|IsValidClass (Variables|Active(usingthesedisablespassiveconversationsforthisNPC!)|GetActiveDialogue))))