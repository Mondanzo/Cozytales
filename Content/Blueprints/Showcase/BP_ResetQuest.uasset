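; An interactable showcase actor that resets quests when the player interacts with it.
; On interact, it loops over its QuestIds array and has the quest manager set each quest to the first status enum value.
; It supplies "Reset Quests" as its interaction display text.
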(event EventBeginPlay
  (|CallParentFunction) ; This node is disabled and will not be called.\nDrag off pins to build functionality.
)

(event Collision|EventActorBeginOverlap
  (params (OtherActor :type Actor%20Object%20Reference))
  (|CallParentFunction OtherActor) ; This node is disabled and will not be called.\nDrag off pins to build functionality.
)

(event EventOnInteract
  (params (Interactor :type Object%20Object%20Reference))
  (for _array_element (Variables|Default|GetQuestIds)
    (Default|UpdateQuestStatus (CallFunction|GetQuestManager) _array_element "NewEnumerator0")))

(fn ConstructionScript
  (|CallParentFunction))

(fn GetDisplayText
  (return "Reset Quests"))