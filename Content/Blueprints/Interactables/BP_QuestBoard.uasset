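; BP_QuestBoard is an interactable board where a player places a map to post a quest.
; Interacting while the board is empty reveals a hidden mesh slot, attaches a new map component and passes the player's map to BP_QuestManager.
; The manager's accepted time drives the map's timeout removal and a timer that decrements the board's quest count.
; Despite the slot search, the count check allows only one map at once.
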(event Custom|Event%20OnMapRemovedFromBoard
  (Variables|Default|SetQuestsOnBoard (- (Variables|Default|GetQuestsOnBoard) 1)))

(event Custom|Event%20StartQuestMapWaitTime
  (params (MapRef :type BP%20Questboard%20Map%20Comp%20Object%20Reference))
  (bind _questmanagerref (Variables|Default|GetQuestManagerRef))
  (bind _questacceptedtime (Variables|/Game/Blueprints/Systems/QuestSystem/BP_QuestManager.BP_QuestManager_C|GetQuestAcceptedTime _questmanagerref))
  (Default|EventRemovefromSlotonWaitTimeout MapRef _questacceptedtime)
  (Utilities|Time|SetTimerbyEvent (delegate Custom|Event%20OnMapRemovedFromBoard) _questacceptedtime))

(event EventBeginPlay
  (|CallParentFunction)
  (Utilities|FlowControl|Delay 0.2)
  (bind _returnvalue (Actor|GetActorOfClass "/Game/Blueprints/Systems/QuestSystem/BP_QuestManager.BP_QuestManager_C"))
  (Variables|Default|SetQuestManagerRef _returnvalue))

(event EventOnInteract
  (params (Interactor :type Object%20Object%20Reference))
  (if (not (> (Variables|Default|GetQuestsOnBoard) 0))
    (CallFunction|HandlePlayerInteraction Interactor)))

(fn ConstructionScript
  (|CallParentFunction))

(fn HandlePlayerInteraction
  (params (Interactor :type Object%20Object%20Reference))
  (bind _asbp_player_character (Utilities|Casting|CastToBP_PlayerCharacter Interactor))
  (bind _array_element (Utilities|Array|ForEachLoopwithBreak (Components|GetChildrenComponents (Variables|Default|GetMesh) false) :!label _label)
    (:LoopBody
      (if (not (Variables|/Script/Engine.SceneComponent|GetbVisible _array_element))
        (LocalVariables|SetParentSlot _array_element)
        (goto _label Break)))
    (:Completed
      (Utilities|IsValid (LocalVariables|GetParentSlot)
        (:Is%20Valid
          (Rendering|SetVisibility (LocalVariables|GetParentSlot) true true)
          (bind _returnvalue (AddComponent|AddBPQuestboardMapComp false))
          (Transformation|AttachComponentToComponent _returnvalue (LocalVariables|GetParentSlot) "None" "KeepRelative" "KeepRelative" "KeepRelative" true)
          (Transformation|ResetRelativeTransform _returnvalue)
          (Variables|Default|SetQuestsOnBoard (+ (Variables|Default|GetQuestsOnBoard) 1))
          (Default|EventSetQuestonBoard (Variables|Default|GetQuestManagerRef) (Variables|/Game/Blueprints/Characters/HeroCharacter/BP_PlayerCharacter.BP_PlayerCharacter_C|GetMapRef _asbp_player_character))
          (CallFunction|EventStartQuestMapWaitTime _returnvalue))
        (:Is%20Not%20Valid
          (Development|PrintString "No free slot!"))))))

(fn GetDisplayText
  (return "Place Map"))